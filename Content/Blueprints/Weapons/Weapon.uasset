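; Weapon Blueprint that holds clip and reserve ammo and provides the reload logic for a gun.
; Reload returns false when the clip is already full or the MaxAmmo reserve is empty.
; Otherwise it moves rounds from MaxAmmo into Ammo, up to ClipSize or until the reserve runs out, and returns true.
; The event graph and construction script are empty, so nothing here handles firing, input or animation.
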(fn `Reload`
  (returns (ReloadSuccess :type Boolean))
  (bind _returnvalue (- (`self.ClipSize`) (`self.Ammo`)))
  (if (== (`self.Ammo`) (`self.ClipSize`))
    (return false)
    (elif (== (`self.MaxAmmo`) 0)
      (return false)
      (else
        (if (< _returnvalue (`self.MaxAmmo`))
          (set `self.MaxAmmo` (- (`self.MaxAmmo`) _returnvalue))
          (set `self.Ammo` (`self.ClipSize`))
          (else
            (set `self.Ammo` (+ (`self.MaxAmmo`) (`self.Ammo`)))
            (set `self.MaxAmmo` 0)))
        (return true)))))

(fn `UserConstructionScript`)