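; Enemy AI character that spawns with an AK47 on its WeaponAttach socket and fights with hitscan fire.
; StartShooting loops on the weapon's fire rate, auto-reloads when empty, and Fire line-traces forward to apply damage with muzzle, sound and impact effects.
; Damage drains a shield while half also bleeds into health.
; Death plays an animation, credits the killer's score and asks MainGameMode to respawn players; Threatened focuses on the player.
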(event `self.ReceiveBeginPlay`
  ;[1 1 1] Spawn AK47
  (bind _returnvalue (`|SpawnActorFromClass` "/Game/Blueprints/Weapons/AK47.AK47_C" (`KismetMathLibrary.MakeTransform` (0.0 0.0 0.0)) "Undefined" "OverrideRootScale" null null))
  (bind _output_get (set `self.EquippedWeapon` _returnvalue))
  (`self.K2_AttachToComponent` _output_get (`self.Mesh`) "WeaponAttach" "KeepRelative" "KeepRelative" "KeepRelative" true))

(event `self.ReceiveAnyDamage`
  (params (Damage :type "Float (single-precision)") (DamageType :type "DamageType Object Reference") (InstigatedBy :type "Controller Object Reference") (DamageCauser :type "Actor Object Reference"))
  ;[1 1 1] Damages and death
  (`self.TakeDamage` Damage)
  (if (== (`self.Health`) 0.0)
    (set `self.IsDead` true)
    (`SkeletalMeshComponent.PlayAnimation` (`self.Mesh`) "/Game/Mannequin/Animation/AnimationSequences/death_from_the_front.death_from_the_front" false)
    (`ActorComponent.K2_DestroyComponent` (`self.CapsuleComponent`))
    (`PrimitiveComponent.SetCollisionEnabled` (`self.Mesh`) "NoCollision")
    (`self.StopShooting`)
    (bind _asfpsplayer_state (cast `/Game/Blueprints/Player/FPSPlayerState` (`Controller.PlayerState` InstigatedBy)))
    (`/Game/Blueprints/Player/FPSPlayerState.IncrementScore` _asfpsplayer_state)
    (`KismetSystemLibrary.Delay` 3.43)
    (bind _asmain_game_mode (cast `/Game/Blueprints/Core/GameModes/MainGameMode` (`GameplayStatics.GetGameMode`)))
    (`/Game/Blueprints/Core/GameModes/MainGameMode.RespawnPlayers` _asmain_game_mode)))

(event `StartShooting`
  (bind _equippedweapon (`self.EquippedWeapon`))
  ;[1 1 1] Shooting
  (if (< (`/Game/Blueprints/Weapons/Weapon.Ammo` (`self.EquippedWeapon`)) 1) :!label _label
    (`/Game/Blueprints/Weapons/Weapon.Reload` (`self.EquippedWeapon`))
    (set `self.IsReloading` true)
    (`KismetSystemLibrary.Delay` 3.3)
    (set `self.IsReloading` false)
    (if (`self.IsFiring`)
      (goto _label))
    (elif (or (`self.IsReloading`) (`self.IsDead`))
      _
      (elif (> (`/Game/Blueprints/Weapons/Weapon.Ammo` _equippedweapon) 0)
        (set `self.IsFiring` true)
        (`self.Fire`)
        (`KismetSystemLibrary.Delay` (`/Game/Blueprints/Weapons/Weapon.FireRate` _equippedweapon))
        (if (`self.IsFiring`)
          (goto _label))))))

(event `StopShooting`
  ;[1 1 1] Shooting
  (set `self.IsFiring` false))

(event `Threatened`
  ;[1 1 1] Threatened
  (`AIController.K2_SetFocus` (`AIBlueprintHelperLibrary.GetAIController` self) (`GameplayStatics.GetPlayerCharacter` 0)))

(fn `Fire`
  (bind _returnvalue (`self.K2_GetActorLocation`))
  (bind _equippedweapon (`self.EquippedWeapon`))
  (bind _location (.location (`SceneComponent.GetSocketTransform` (`/Game/Blueprints/Weapons/Weapon.SkeletalMesh` (`self.EquippedWeapon`)) "Muzzle" "RTS_World")))
  (bind _outhit (`KismetSystemLibrary.LineTraceSingle` _returnvalue (+ _returnvalue (* (`KismetMathLibrary.GetForwardVector` (`self.K2_GetActorRotation`)) 8000.0)) "TraceTypeQuery2"))
  (bind (_bblockinghit _binitialoverlap _time _distance _location_2 _impactpoint _normal _impactnormal _physmat _hitactor) (`GameplayStatics.BreakHitResult` _outhit))
  (`GameplayStatics.ApplyDamage` _hitactor (`/Game/Blueprints/Weapons/Weapon.Damage` (`self.EquippedWeapon`)) (`AIBlueprintHelperLibrary.GetAIController` self) self)
  (set `/Game/Blueprints/Weapons/Weapon.Ammo` (- (`/Game/Blueprints/Weapons/Weapon.Ammo` _equippedweapon) 1) _equippedweapon)
  (`GameplayStatics.SpawnEmitterAtLocation` "/Game/Weapons/Particles/MFParticles.MFParticles" _location (.rotation (`SceneComponent.GetSocketTransform` (`/Game/Blueprints/Weapons/Weapon.SkeletalMesh` (`self.EquippedWeapon`)) "Muzzle" "RTS_World")) (0.05 0.05 0.05))
  (`GameplayStatics.PlaySoundAtLocation` (`/Game/Blueprints/Weapons/Weapon.FireFX` (`self.EquippedWeapon`)) _location (struct) 0.2 1.0 0.0 "/Game/Audio/SoundAttenuation.SoundAttenuation" null null)
  (if _bblockinghit
    (`GameplayStatics.SpawnEmitterAtLocation` "/Game/Weapons/Particles/ImpactParticles.ImpactParticles" _location_2)))

(fn `TakeDamage`
  (params (Damage :type "Float (double-precision)"))
  (bind _output_get (set `self.Shield` (- (`self.Shield`) Damage)))
  (if (< _output_get 0.0)
    (bind _output_get_2 (set `self.Health` (+ (`self.Shield`) (`self.Health`))))
    (set `self.Shield` 0.0)
    (if (< _output_get_2 0.0)
      (set `self.Health` 0.0))
    (else
      (bind _output_get_3 (set `self.Health` (- (`self.Health`) (* Damage 0.5))))
      (if (< _output_get_3 0.0)
        (set `self.Health` 0.0)))))

(fn `UserConstructionScript`)