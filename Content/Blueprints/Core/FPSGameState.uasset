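; FPSGameState is a game state Blueprint that runs the round-start countdown.
; StartRoundTimer loops on a one-second Delay, decrementing Countdown until it reaches 1.
; It then calls RemoveStartRoundTimer on each FPSPlayerController in the FPSGameMode's PlayerControllers list and resets Countdown to 5 inside that loop.
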(event `StartRoundTimer`
  (`KismetSystemLibrary.Delay` 1.0 :!label _label)
  (if (== (`self.Countdown`) 1)
    (bind _asfpsgame_mode (cast `/Game/Blueprints/Core/GameModes/FPSGameMode` (`GameplayStatics.GetGameMode`)))
    (for _array_element (`/Game/Blueprints/Core/GameModes/FPSGameMode.PlayerControllers` _asfpsgame_mode)
      (bind _asfpsplayer_controller (cast `/Game/Blueprints/Player/FPSPlayerController` _array_element))
      (`/Game/Blueprints/Player/FPSPlayerController.RemoveStartRoundTimer` _asfpsplayer_controller)
      (set `self.Countdown` 5))
    (else
      (set `self.Countdown` (- (`self.Countdown`) 1))
      (goto _label))))

(fn `UserConstructionScript`)