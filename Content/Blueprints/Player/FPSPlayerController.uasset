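; Player controller for the FPS that owns the match UI: scope parent, waiting-players screen, round-start timer, scoreboard and end screen.
; Events create each widget, keep a reference, push data into it, and remove the waiting screen and timer on request.
; Screens toggle cursor or input mode as needed.
; The end screen copies server and client names and scores from the scoreboard, which it then replaces.
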(event `Add Scope Parent`
  ;[1 1 1] Add scope parent widget to viewport (scope hud will be add to "scope parent")
  (bind _returnvalue (`|CreateWidget` "/Game/UI/ScopeParentHUD.ScopeParentHUD_C"))
  (bind _output_get (set `self.ScopeParentRef` _returnvalue))
  (`UserWidget.AddToViewport` _output_get 0))

(event `DisplayWaitingPlayers`
  ;[1 1 1] Waiting Players Screen (display/remove/update)
  (bind _returnvalue (`|CreateWidget` "/Game/UI/WaitingPlayersScreen.WaitingPlayersScreen_C"))
  (bind _output_get (set `self.WaitingPlayerRef` _returnvalue))
  (`UserWidget.AddToViewport` _output_get 0)
  (set `self.bShowMouseCursor` true))

(event `RemoveWaitingPlayers`
  (bind _waitingplayerref (`self.WaitingPlayerRef`))
  ;[1 1 1] Waiting Players Screen (display/remove/update)
  (`/Engine/EditorBlueprintResources/StandardMacros.IsValid` _waitingplayerref
    (:`Is Valid`
      (`Widget.RemoveFromParent` _waitingplayerref)
      (set `self.bShowMouseCursor` false))))

(event `UpdateNumberPlayersLogged`
  (params (NumberPlayersLogged :type Integer))
  ;[1 1 1] Waiting Players Screen (display/remove/update)
  (set `/Game/UI/WaitingPlayersScreen.NumberPlayersLogged` NumberPlayersLogged (`self.WaitingPlayerRef`)))

(event `DisplayStartRoundTimer`
  ;[1 1 1] Start Round Timer Widget (display/remove)
  (bind _returnvalue (`|CreateWidget` "/Game/UI/StartRoundTimer.StartRoundTimer_C"))
  (bind _output_get (set `self.StartRoundTimerRef` _returnvalue))
  (`UserWidget.AddToViewport` _output_get 0)
  (`WidgetBlueprintLibrary.SetInputMode_UIOnlyEx` self _output_get))

(event `RemoveStartRoundTimer`
  (bind _startroundtimerref (`self.StartRoundTimerRef`))
  ;[1 1 1] Start Round Timer Widget (display/remove)
  (`/Engine/EditorBlueprintResources/StandardMacros.IsValid` _startroundtimerref
    (:`Is Valid`
      (`Widget.RemoveFromParent` _startroundtimerref)
      (`WidgetBlueprintLibrary.SetInputMode_GameOnly` self))))

(event `DisplayScoreboard`
  ;[1 1 1] Scoreboard Widget
  (bind _returnvalue (`|CreateWidget` "/Game/UI/Scoreboard.Scoreboard_C"))
  (bind _output_get (set `self.ScoreboardRef` _returnvalue))
  (`UserWidget.AddToViewport` _output_get 0))

(event `UpdateScore`
  (params (ServerScore :type Integer) (ClientScore :type Integer) (ServerPlayerName :type Text) (ClientPlayerName :type Text))
  (bind _scoreboardref (`self.ScoreboardRef`))
  ;[1 1 1] Scoreboard Widget
  (set `/Game/UI/Scoreboard.ServerScore` ServerScore _scoreboardref)
  (set `/Game/UI/Scoreboard.ClientScore` ClientScore _scoreboardref)
  (set `/Game/UI/Scoreboard.ServerPlayerName` ServerPlayerName _scoreboardref)
  (set `/Game/UI/Scoreboard.ClientPlayerName` ClientPlayerName _scoreboardref))

(event `DisplayEndScreen`
  (params (IsADraw :type Boolean) (HasServerWon :type Boolean))
  (bind _scoreboardref (`self.ScoreboardRef`))
  ;[1 1 1] End Screen
  (bind _returnvalue (`|CreateWidget` "/Game/UI/EndScreen.EndScreen_C"))
  (bind _output_get (set `self.EndScreenRef` _returnvalue))
  (set `/Game/UI/EndScreen.IsADraw` IsADraw _output_get)
  (set `/Game/UI/EndScreen.HasServerWon` HasServerWon _output_get)
  (set `/Game/UI/EndScreen.ServerScore` (`/Game/UI/Scoreboard.ServerScore` _scoreboardref) _output_get)
  (set `/Game/UI/EndScreen.ClientScore` (`/Game/UI/Scoreboard.ClientScore` _scoreboardref) _output_get)
  (set `/Game/UI/EndScreen.ServerPlayerName` (`/Game/UI/Scoreboard.ServerPlayerName` _scoreboardref) _output_get)
  (set `/Game/UI/EndScreen.ClientPlayerName` (`/Game/UI/Scoreboard.ClientPlayerName` _scoreboardref) _output_get)
  (`Widget.RemoveFromParent` _scoreboardref)
  (`UserWidget.AddToViewport` _output_get 0)
  (`WidgetBlueprintLibrary.SetInputMode_UIOnlyEx` self _output_get)
  (set `self.bShowMouseCursor` true))

(fn `UserConstructionScript`)